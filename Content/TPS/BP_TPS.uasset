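; Third-person shooter player character with movement, jump, crouch, prone, stamina-limited sprint and aimed shooting.
; Right mouse plays a weapon-hold montage and a timeline FOV zoom; left mouse then line-traces from the camera, flagging any hit BP_Enemy dead.
; Tick drains or refills stamina and cancels aim montages during sprint or prone.
; BeginPlay adds the WBP_TPS HUD and starts looping timers for an elapsed-time counter and its padded seconds string.
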(event Custom|MillisecondTick
  ;[1 1 1] Timer
  (if (not (Variables|Default|GetStopTimer))
    (Variables|Default|SetMillisecond (+ (Variables|Default|GetMillisecond) 1))
    (if (> (Variables|Default|GetMillisecond) 999)
      (Math|Integer|IncrementInt (Variables|Default|GetTimeSecond)
        (:%20%20
          (Variables|Default|SetMillisecond 0))))))

(event Custom|SecondCheck
  ;[1 1 1] SecondDisplay
  (Variables|Default|SetSecondStringDisplay "000")
  (if (< (Variables|Default|GetTimeSecond) 10)
    (Variables|Default|SetSecondStringDisplay (Utilities|String|Append "00" (Utilities|String|ToString(Integer) (Variables|Default|GetTimeSecond))))
    (elif (< (Variables|Default|GetTimeSecond) 100)
      (Variables|Default|SetSecondStringDisplay (Utilities|String|Append "0" (Utilities|String|ToString(Integer) (Variables|Default|GetTimeSecond))))
      (else
        (Variables|Default|SetSecondStringDisplay (Utilities|String|ToString(Integer) (Variables|Default|GetTimeSecond)))))))

(event Custom|SprintValueModification
  ;[1 1 1] StaminaBar
  (if (Variables|Default|GetSprintButtonPressed)
    (Variables|Default|SetSprintValue (Math|Float|Clamp(Float) (- (Variables|Default|GetSprintValue) 0.005)))
    (else
      (Variables|Default|SetSprintValue (Math|Float|Clamp(Float) (+ (Variables|Default|GetSprintValue) 0.005))))))

(event Custom|ToogleCanSprint
  ;[1 1 1] ToolgeCanSprint
  (if (> (Variables|Default|GetSprintValue) 0.0)
    (Variables|Default|SetCanSprint true)
    (else
      (Variables|Default|SetCanSprint false)
      (Variables|Default|SetSprintButtonPressed false)
      (if (not (or (Variables|Default|GetWSPressed) (Variables|Default|GetADPressed)))
        (Variables|/Script/Engine.CharacterMovementComponent|SetMaxWalkSpeed (Variables|Character|GetCharacterMovement) 0.0)))))

(event EventTick
  (params (DeltaSeconds :type Float%20%28single-precision%29))
  ;[1 1 1] Already aiming stop when start sprinting
  (CallFunction|SprintValueModification)
  (CallFunction|ToogleCanSprint)
  (if (or (Variables|Default|GetSprintButtonPressed) (Variables|Default|GetProneButtonPressed))
    (Animation|StopAnimMontage "/Game/TPS/M_TPS_WeaponHoldCrouch.M_TPS_WeaponHoldCrouch")
    (Animation|StopAnimMontage "/Game/TPS/M_TPS_WeaponHoldNormal.M_TPS_WeaponHoldNormal")))

(event EventBeginPlay
  (bind _returnvalue (UserInterface|CreateWidget "/Game/TPS/WBP_TPS.WBP_TPS_C"))
  (UserInterface|Viewport|AddtoViewport _returnvalue 0)
  ;[1 1 1] Set Timer (TimerFunction / SecondDisplay)
  (Utilities|Time|SetTimerbyFunctionName 0 "MillisecondTick" 0.001 true)
  (Utilities|Time|SetTimerbyFunctionName 0 "SecondCheck" 0.001 true))

(event Input|ActionEvents|InputActionJump
  (params (Key :type Key%20Structure))
  ;[1 1 1] Jumping
  (:Pressed
    (Character|Jump)
    (Variables|Default|SetJumping%20Pressed true))
  (:Released
    (Character|StopJumping)
    (Variables|Default|SetJumping%20Pressed false)))

(event Input|AxisEvents|InputAxisTurn
  (params (AxisValue :type Float%20%28single-precision%29))
  ;[1 1 1] MouseControl
  (Pawn|Input|AddControllerYawInput AxisValue))

(event Input|AxisEvents|InputAxisLookUp
  (params (AxisValue :type Float%20%28single-precision%29))
  ;[1 1 1] MouseControl
  (Pawn|Input|AddControllerPitchInput AxisValue))

(event Input|AxisEvents|InputAxisMoveForward
  (params (AxisValue :type Float%20%28single-precision%29))
  ;[1 1 1] Movement ( AWSD or Joystick)
  (if (!= AxisValue 0.0)
    (Variables|Default|SetWSPressed true)
    (else
      (Variables|Default|SetWSPressed false)))
  (if (and (not (Variables|Default|GetSprintButtonPressed)) (not (Variables|Default|GetProneButtonPressed)))
    (if (Variables|Default|GetCanMove)
      (Pawn|Input|AddMovementInput (Math|Vector|GetForwardVector (Math|Rotator|MakeRotator 0.0 0.0 (.Yaw (Math|Rotator|BreakRotator (Pawn|GetControlRotation :!class /Script/Engine.Pawn))))) (.X (Math|Vector|BreakVector (Math|Vector|Normalize (Math|Vector|MakeVector AxisValue (stale Input|AxisEvents|InputAxisMoveRight AxisValue) 0.0)))) false))))

(event Input|AxisEvents|InputAxisMoveRight
  (params (AxisValue :type Float%20%28single-precision%29))
  ;[1 1 1] Movement ( AWSD or Joystick)
  (if (!= AxisValue 0.0)
    (Variables|Default|SetADPressed true)
    (else
      (Variables|Default|SetADPressed false)))
  (if (and (not (Variables|Default|GetSprintButtonPressed)) (not (Variables|Default|GetProneButtonPressed)))
    (if (Variables|Default|GetCanMove)
      (Pawn|Input|AddMovementInput (Math|Vector|GetRightVector (Math|Rotator|MakeRotator 0.0 0.0 (.Yaw (Math|Rotator|BreakRotator (Pawn|GetControlRotation :!class /Script/Engine.Pawn))))) (.Y (Math|Vector|BreakVector (Math|Vector|Normalize (Math|Vector|MakeVector (stale Input|AxisEvents|InputAxisMoveForward AxisValue) AxisValue 0.0)))) false))))

(event Input|AxisEvents|InputAxisSprint
  (params (AxisValue :type Float%20%28single-precision%29))
  ;[1 1 1] Sprint
  (if (and (not (Variables|Default|GetCrouchButtonPressed)) (not (Variables|Default|GetProneButtonPressed)))
    (if (Variables|Default|GetCanMove)
      (if (Variables|Default|GetCanSprint)
        (Pawn|Input|AddMovementInput (Math|Vector|GetForwardVector (Math|Rotator|MakeRotator 0.0 0.0 (.Yaw (Math|Rotator|BreakRotator (Pawn|GetControlRotation :!class /Script/Engine.Pawn))))) AxisValue false)))))

(event Input|KeyboardEvents|LeftCtrl
  (params (Key :type Key%20Structure))
  (bind _mesh (Variables|Character|GetMesh))
  (bind _rightmousebuttonpressed (Variables|Default|GetRightMouseButtonPressed))
  ;[1 1 1] Crouch
  (:Pressed
    (Variables|Default|SetCrouchButtonPressed true)
    (Character|Crouch)
    (if (Variables|Default|GetSprintButtonPressed)
      (Variables|Default|SetSprintButtonPressed false)
      (if _rightmousebuttonpressed
        (Animation|Montage|PlayMontage _mesh "/Game/TPS/M_TPS_WeaponHoldCrouch.M_TPS_WeaponHoldCrouch"))))
  (:Released
    (Variables|Default|SetCrouchButtonPressed false)
    (Character|UnCrouch)
    (if _rightmousebuttonpressed
      (Animation|Montage|PlayMontage _mesh "/Game/TPS/M_TPS_WeaponHoldNormal.M_TPS_WeaponHoldNormal"))))

(event Input|MouseEvents|RightMouseButton
  (params (Key :type Key%20Structure))
  (bind _mesh (Variables|Character|GetMesh))
  ;[1 1 1] Aiming( Normal/Crouching)
  (:Pressed
    (if (and (not (Variables|Default|GetSprintButtonPressed)) (not (Variables|Default|GetProneButtonPressed)))
      (Variables|Default|SetRightMouseButtonPressed true)
      (if (Variables|Default|GetCrouchButtonPressed)
        (Animation|Montage|PlayMontage _mesh "/Game/TPS/M_TPS_WeaponHoldCrouch.M_TPS_WeaponHoldCrouch"
          (:then
            ;[1 1 1] Aim Zoom in and Zoom out
            (bind _newtrack_0 (Timeline|Timeline_0 Play)
              (:Update
                (Camera|SetFieldOfView (Variables|Default|GetCamera) (Math|Float|Lerp 9e+01 45.0 _newtrack_0))))))
        (else
          (Animation|Montage|PlayMontage _mesh "/Game/TPS/M_TPS_WeaponHoldNormal.M_TPS_WeaponHoldNormal"
            (:then
              (Timeline|Timeline_0 Play)))))))
  (:Released
    (Variables|Default|SetRightMouseButtonPressed false)
    (if (Variables|Default|GetCrouchButtonPressed)
      (Animation|StopAnimMontage "/Game/TPS/M_TPS_WeaponHoldCrouch.M_TPS_WeaponHoldCrouch")
      (Timeline|Timeline_0 Reverse)
      (else
        (Animation|StopAnimMontage "/Game/TPS/M_TPS_WeaponHoldNormal.M_TPS_WeaponHoldNormal")
        (Timeline|Timeline_0 Reverse)))))

(event Input|KeyboardEvents|LeftShift
  (params (Key :type Key%20Structure))
  (bind _charactermovement (Variables|Character|GetCharacterMovement))
  ;[1 1 1] Sprint
  (:Pressed
    (if (not (Variables|Default|GetCrouchButtonPressed))
      (if (Variables|Default|GetCanSprint)
        (Variables|/Script/Engine.CharacterMovementComponent|SetMaxWalkSpeed _charactermovement 9e+02)
        (Variables|Default|SetSprintButtonPressed true))))
  (:Released
    (Variables|/Script/Engine.CharacterMovementComponent|SetMaxWalkSpeed _charactermovement 6e+02)
    (Variables|Default|SetSprintButtonPressed false)))

(event Input|MouseEvents|LeftMouseButton
  (params (Key :type Key%20Structure))
  (bind _camera (Variables|Default|GetCamera))
  (bind _returnvalue (Transformation|GetWorldLocation _camera))
  ;[1 1 1] Linetrace
  (:Pressed
    (if (Variables|Default|GetRightMouseButtonPressed)
      (Variables|Default|SetShootPressed true)
      (bind _outhit (Collision|LineTraceByChannel _returnvalue (+ _returnvalue (* (Math|Vector|GetForwardVector (Transformation|GetWorldRotation _camera)) 1e+04)) "TraceTypeQuery1" false 0 "ForDuration"))
      (bind _asbp_enemy (Utilities|Casting|CastToBP_Enemy (.HitActor (Collision|BreakHitResult _outhit))))
      (Variables|/Game/TPS/BP_Enemy.BP_Enemy_C|SetIsDeath _asbp_enemy true)))
  (:Released
    (Variables|Default|SetShootPressed false)))

(event Input|KeyboardEvents|C
  (params (Key :type Key%20Structure))
  ;[1 1 1] Prone
  (:Pressed
    (Variables|Default|SetProneButtonPressed true)
    (Variables|Default|SetCanMove false))
  (:Released
    (Variables|Default|SetProneButtonPressed false)))

(fn ConstructionScript)