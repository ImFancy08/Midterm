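; BP_Enemy is a TPS enemy Blueprint that keeps turning to face the player while it is alive.
; Each Tick, while IsDeath is false, it snaps its rotation to the look-at yaw toward player character 0, with pitch and roll zeroed.
; The same Tick rerolls DeathNumber among three values, though nothing in this graph reads it or sets IsDeath to true.
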(event EventBeginPlay
  (Variables|Default|SetIsDeath false))

(event EventTick
  (params (DeltaSeconds :type Float%20%28single-precision%29))
  (if (not (Variables|Default|GetIsDeath))
    (Variables|Default|SetDeathNumber (Math|Random|RandomIntegerinRange 0 2))
    (Transformation|SetActorRotation (Math|Rotator|MakeRotator 0.0 0.0 (.Yaw (Math|Rotator|BreakRotator (Math|Rotator|FindLookatRotation (Transformation|GetActorLocation) (Transformation|GetActorLocation (Game|GetPlayerCharacter 0)))))))))

(fn ConstructionScript)